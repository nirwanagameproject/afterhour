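; Zombie captain enemy that chases the first-person player on sight and catches them in a jumpscare-style sequence.
; Sight perception sets CanSeePlayer, and Tick fires a once-per-sighting switch to the attack state, which updates the Blackboard and walk speed, plus an AIMoveTo.
; CatchBox overlap stops movement and disables input while a timeline turns the player's view to the zombie, then snaps it in front of them under a spotlight.
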(event OnTargetPerceptionUpdated(AIPerceptionsight)
  (params (Actor :type Actor%20Object%20Reference) (Stimulus :type AI%20Stimulus%20Structure))
  ;[1 1 1] Set Variable CanSeePlayer
  (Utilities|FlowControl|Sequence
    (:then_1
      (Utilities|Casting|CastToBP_FirstPersonCharacter Actor)
      (Variables|Default|SetCanSeePlayer (.bSuccessfullySensed (Utilities|Struct|BreakAIStimulus Stimulus))))))

(event OnComponentBeginOverlap(CatchBox)
  (params (OverlappedComponent :type Primitive%20Component%20Object%20Reference) (OtherActor :type Actor%20Object%20Reference) (OtherComp :type Primitive%20Component%20Object%20Reference) (OtherBodyIndex :type Integer) (bFromSweep :type Boolean) (SweepResult :type Hit%20Result%20Structure%20%28by%20ref%29))
  ;[1 1 1] Collsion Beetween Player and Enemy
  (Utilities|Casting|CastToBP_FirstPersonCharacter OtherActor)
  (if (Variables|Default|GetCanCatch)
    (CallFunction|CatchPlayer)
    (Pawn|Components|CharacterMovement|SetMovementMode (Variables|Character|GetCharacterMovement) "MOVE_None" 0)))

(event Custom|CatchPlayer
  (bind _returnvalue (Game|GetPlayerController 0))
  (bind _returnvalue_2 (Game|GetPlayerCharacter 0))
  (bind _returnvalue_3 (Game|GetPlayerCharacter 0))
  ;[1 1 1] CatchPlayer Event
  (Utilities|FlowControl|Sequence
    (:then_0
      (bind _alpha (Timeline|PlayerLookAt PlayFromStart)
        (:Update
          (if (Variables|Default|GetCanCatch)
            (Pawn|SetControlRotation _returnvalue (Math|Rotator|Lerp(Rotator) (Pawn|GetControlRotation _returnvalue :!class /Script/Engine.Controller) (Math|Rotator|FindLookatRotation (Transformation|GetActorLocation _returnvalue_3) (Transformation|GetActorLocation)) _alpha true))
            (else
              (Timeline|PlayerLookAt Stop))))
        (:Finished
          (if (Variables|Default|GetCanCatch)
            (Transformation|SetActorLocation (+ (+ (Transformation|GetActorLocation _returnvalue_2) (* (Transformation|GetActorForwardVector _returnvalue_2) 2.5)) "0,0.000000,-15.000000") false false)
            (Rendering|SetVisibility (Variables|Default|GetSpotLight) true false)
            (Variables|Default|SetCanCatch false)))))
    (:then_1
      (Input|DisableInput _returnvalue_3 (Game|GetPlayerController 0)))))

(event EventBeginPlay)

(event Collision|EventActorBeginOverlap
  (params (OtherActor :type Actor%20Object%20Reference)))

(event EventTick
  (params (DeltaSeconds :type Float%20%28single-precision%29))
  ;[1 1 1] Move Event When Enemy See Player
  (if (Variables|Default|GetCanSeePlayer)
    (Utilities|FlowControl|DoOnce false :!label _label
      (:Completed
        (CallFunction|SetState "NewEnumerator2")
        (AI|AIMoveTo self "0, 0, 0" (Game|GetPlayerCharacter 0) 0.0 false)))
    (else
      (goto _label Reset))))

(fn ConstructionScript)

(fn SetState
  (params (NewState :type ZombieState%20Enum :default "NewEnumerator0"))
  (bind _charactermovement (Variables|Character|GetCharacterMovement))
  (AI|Components|Blackboard|SetValueasEnum (AI|GetBlackboard 0) (Utilities|Name|MakeLiteralName "State") NewState)
  (switch Utilities|FlowControl|Switch|SwitchonZombieState NewState
    (:NewEnumerator0
      (Variables|/Script/Engine.CharacterMovementComponent|SetMaxWalkSpeed _charactermovement 25.0))
    (:NewEnumerator1
      (Variables|/Script/Engine.CharacterMovementComponent|SetMaxWalkSpeed _charactermovement 5e+01))
    (:NewEnumerator2
      (Variables|/Script/Engine.CharacterMovementComponent|SetMaxWalkSpeed _charactermovement 1e+02))))